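; Player spider character that moves along world Y, jumps and wall-jumps, interacts with objects and knocks back enemies.
; Tick traces to both Y sides, so Space launches the character when airborne beside a "wall"-tagged actor, otherwise jumps.
; F messages the first overlapping InteractInterface actor; OverlapBox tracks a BaseEnemy for the A action's knockback.
; Climbing, vertical movement and facing updates are disconnected.
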(event `self.ReceiveBeginPlay`)

(event `InputAxis|Horizontal`
  (params (AxisValue :type "Float (single-precision)"))
  (`self.AddMovementInput` (`KismetMathLibrary.MakeVector` 0.0 (`self.Speed`)) AxisValue))

(event `InputAxis|Vertical`
  (params (AxisValue :type "Float (single-precision)")))

(event `Key|F`
  (params (Key :type "Key Structure"))
  (:`Pressed`
    (for _array_element (`self.GetOverlappingActors` "/Script/Engine.Actor")
      (if (`KismetSystemLibrary.DoesImplementInterface` _array_element "/Game/Blueprints/DoorA/InteractInterface.InteractInterface_C")
        (message `/Game/Blueprints/DoorA/InteractInterface.Interact` _array_element self)
        (break)))))

(event `Knockback`)

(event `self.ReceiveTick`
  (params (DeltaSeconds :type "Float (single-precision)"))
  (bind _returnvalue (`SceneComponent.K2_GetComponentLocation` (`self.CapsuleComponent`)))
  (bind _returnvalue_2 (`SceneComponent.K2_GetComponentLocation` (`self.CapsuleComponent`)))
  (bind (_x _y _z) (`KismetMathLibrary.BreakVector3f` _returnvalue))
  (bind (_x_2 _y_2 _z_2) (`KismetMathLibrary.BreakVector3f` _returnvalue_2))
  (`|ExecutionSequence`
    (:`then_0`
      (bind _outhit (`KismetSystemLibrary.LineTraceSingle` _returnvalue_2 (`KismetMathLibrary.MakeVector` _x_2 (+ _y_2 50.0) _z_2) "TraceTypeQuery1")))
    (:`then_1`
      (bind _outhit_2 (`KismetSystemLibrary.LineTraceSingle` _returnvalue (`KismetMathLibrary.MakeVector` _x (- _y 50.0) _z) "TraceTypeQuery1")))))

(event `self.OverlapBox.OnComponentBeginOverlap`
  (params (OverlappedComponent :type "PrimitiveComponent Object Reference") (OtherActor :type "Actor Object Reference") (OtherComp :type "PrimitiveComponent Object Reference") (OtherBodyIndex :type Integer) (bFromSweep :type Boolean) (SweepResult :type "HitResult Structure (by ref)"))
  (bind _asbase_enemy (cast `/Game/Blueprints/BaseEnemy` OtherActor))
  (set `self.HitCheck` true))

(event `Key|SpaceBar`
  (params (Key :type "Key Structure"))
  (bind (_forwardvector_x _forwardvector_y _forwardvector_z) (`KismetMathLibrary.BreakVector` (`self.ForwardVector`)))
  (:`Pressed`
    (if (and (or (`self.ActorHasTag` (`.HitActor` (`GameplayStatics.BreakHitResult` (stale `self.ReceiveTick` _outhit))) "wall") (`self.ActorHasTag` (`.HitActor` (`GameplayStatics.BreakHitResult` (stale `self.ReceiveTick` _outhit_2))) "wall")) (`NavMovementComponent.IsFalling` (`self.CharacterMovement`)))
      (`KismetSystemLibrary.PrintString` "WallJump")
      (`self.LaunchCharacter` (`KismetMathLibrary.MakeVector` _forwardvector_x (* _forwardvector_y -800.0) (+ _forwardvector_z 1600.0)))
      (else
        (`self.Jump`))))
  (:`Released`
    (`self.StopJumping`)))

(event `self.OverlapBox.OnComponentEndOverlap`
  (params (OverlappedComponent :type "PrimitiveComponent Object Reference") (OtherActor :type "Actor Object Reference") (OtherComp :type "PrimitiveComponent Object Reference") (OtherBodyIndex :type Integer))
  (cast `/Game/Blueprints/BaseEnemy` OtherActor)
  (set `self.HitCheck` false))

(event `InputAction|A`
  (params (Key :type "Key Structure"))
  (:`Pressed`
    (if (`self.HitCheck`)
      (`/Game/Blueprints/BaseEnemy.knockback` (stale `self.OverlapBox.OnComponentBeginOverlap` _asbase_enemy)))))

(fn `ClimbingLineTrace`
  (returns (OutHit :type "HitResult Structure") (HasHit :type Boolean))
  (bind _returnvalue (`self.K2_GetActorLocation`))
  (bind (_outhit _returnvalue_2) (`KismetSystemLibrary.LineTraceSingle` :`Start` _returnvalue :`End` (+ _returnvalue (* (`KismetMathLibrary.GetForwardVector` (`self.K2_GetActorRotation`)) 100.0)) :`TraceChannel` "TraceTypeQuery1" :`DrawDebugType` "ForDuration"))
  (return _outhit _returnvalue_2))

(fn `UserConstructionScript`)