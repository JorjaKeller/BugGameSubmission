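; CharacterAnt is a player character Blueprint for an ant that moves along the world Y axis, jumps, interacts and knocks back enemies.
; Horizontal input moves it and flips OverlapBox to the facing side, where overlaps flag a BaseEnemy that the A action knocks back.
; F sends InteractMessage to the first overlapping actor implementing InteractInterface.
; Vertical movement is disconnected, and the per-tick downward ground trace drives nothing.
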(event `MoveRight`
  (`KismetSystemLibrary.PrintString` (`KismetStringLibrary.Conv_IntToString` (`self.NewVar`))))

(event `self.ReceiveBeginPlay`)

(event `InputAxis|Horizontal`
  (params (AxisValue :type "Float (single-precision)"))
  (bind _overlapbox (`self.OverlapBox`))
  (`self.AddMovementInput` (`KismetMathLibrary.MakeVector` 0.0 (`self.Speed`)) AxisValue)
  (if (> AxisValue 0.0)
    (`SceneComponent.K2_SetRelativeLocation` _overlapbox (0.0 90.0 0.0) false false)
    (set `self.ForwardVector` (0.0 1.0 0.0))
    (elif (< AxisValue 0.0)
      (`SceneComponent.K2_SetRelativeLocation` _overlapbox (0.0 -90.0 0.0) false false)
      (set `self.ForwardVector` (0.0 -1.0 0.0)))))

(event `InputAxis|Vertical`
  (params (AxisValue :type "Float (single-precision)")))

(event `Key|F`
  (params (Key :type "Key Structure"))
  (:`Pressed`
    (for _array_element (`self.GetOverlappingActors` "/Script/Engine.Actor")
      (if (`KismetSystemLibrary.DoesImplementInterface` _array_element "/Game/Blueprints/DoorA/InteractInterface.InteractInterface_C")
        (message `/Game/Blueprints/DoorA/InteractInterface.Interact` _array_element self)
        (break)))))

(event `Key|SpaceBar`
  (params (Key :type "Key Structure"))
  (:`Pressed`
    (`self.Jump`)))

(event `Knockback`)

(event `self.ReceiveTick`
  (params (DeltaSeconds :type "Float (single-precision)"))
  (bind _returnvalue (`SceneComponent.K2_GetComponentLocation` (`self.CapsuleComponent`)))
  (bind _outhit (`KismetSystemLibrary.LineTraceSingle` _returnvalue (- _returnvalue (0.0 0.0 100.0)) "TraceTypeQuery1"))
  (if true
    _))

(event `self.OverlapBox.OnComponentBeginOverlap`
  (params (OverlappedComponent :type "PrimitiveComponent Object Reference") (OtherActor :type "Actor Object Reference") (OtherComp :type "PrimitiveComponent Object Reference") (OtherBodyIndex :type Integer) (bFromSweep :type Boolean) (SweepResult :type "HitResult Structure (by ref)"))
  (bind _asbase_enemy (cast `/Game/Blueprints/BaseEnemy` OtherActor))
  (set `self.HitCheck` true))

(event `self.OverlapBox.OnComponentEndOverlap`
  (params (OverlappedComponent :type "PrimitiveComponent Object Reference") (OtherActor :type "Actor Object Reference") (OtherComp :type "PrimitiveComponent Object Reference") (OtherBodyIndex :type Integer))
  (cast `/Game/Blueprints/BaseEnemy` OtherActor)
  (set `self.HitCheck` false))

(event `self.OnJumped`)

(event `InputAction|A`
  (params (Key :type "Key Structure"))
  (:`Pressed`
    (if (`self.HitCheck`)
      (`/Game/Blueprints/BaseEnemy.knockback` (stale `self.OverlapBox.OnComponentBeginOverlap` _asbase_enemy)))))

(fn `UserConstructionScript`)